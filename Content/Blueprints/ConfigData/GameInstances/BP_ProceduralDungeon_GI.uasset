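; Game instance Blueprint for procedural dungeon setup, which picks a seed and spawns the starting room through InitializeDungeonIF.
; A LoadingSeed of zero randomizes SeedStream and stores the resulting seed; the step applying a nonzero seed is not connected.
; The starter room class is drawn from StartRoomClasses using SeedStream, with a length-minus-one Max, and spawned at StartRoomSpawnPoint.
; Unconnected random-stream nodes remain as reference.
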(event EventInitializeDungeonIF
  (CallFunction|ProcessSeedInput)
  (CallFunction|GenerateStarterRoom))

(fn ProcessSeedInput
  (if (== (Variables|Default|GetLoadingSeed) 0) ; If the user inputted 0 as their\ndesired seed, then it will ignore\nthe input, and the seed will be\nrandomized.\n\nIf the user did not input 0,\nthen the inputted number will be\nset as the seed number moving forward.
    (Class|KismetMathLibrary|SeedRandomStream (Variables|Default|GetSeedStream)) ; Similar to a variable Setter, but with\nmore functionality.\nThis sets the random seed to be a\nrandom value.
    (Variables|Default|SetLoadingSeed (.initialseed (Variables|Default|GetSeedStream))) ; Used as a reference of the seed...
  ))

(fn GenerateStarterRoom
  (Game|SpawnActorfromClass (CallFunction|RandomizeStarterRoom) (Variables|Default|GetStartRoomSpawnPoint) "Undefined" "MultiplyWithRoot" 0 0) ; Spawns in the starting room
)

(fn RandomizeStarterRoom
  (bind _startroomclasses (Variables|Default|GetStartRoomClasses))
  (return (Utilities|Array|Get(acopy) _startroomclasses (Class|KismetMathLibrary|RandomIntegerfromStream (Variables|Default|GetSeedStream) (- (Utilities|Array|Length _startroomclasses) 1)))))